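; BP_EnemyBoss is a boss enemy that fires projectile volleys at the player and summons melee minions.
; A trigger box starts the Blackboard attack and creates the HUD boss life bar.
; Attack and invoke events play montages, and BeginPlay binds anim Blueprint dispatchers for attack and summon timing.
; Functions spawn projectiles at random navigable points, launch them at the player, and spawn minions with random waypoints.
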(event OnComponentBeginOverlap(Box)
  (params (OverlappedComponent :type Primitive%20Component%20Object%20Reference) (OtherActor :type Actor%20Object%20Reference) (OtherComp :type Primitive%20Component%20Object%20Reference) (OtherBodyIndex :type Integer) (bFromSweep :type Boolean) (SweepResult :type Hit%20Result%20Structure%20%28by%20ref%29))
  (Utilities|Casting|CastToBP_FirstPersonCharacter OtherActor)
  (AI|Components|Blackboard|SetValueasBool (Variables|Default|GetBlackBoard) (Variables|Default|GetStartAttack) true)
  (bind _asbp_custom_hud (Utilities|Casting|CastToBP_CustomHUD (HUD|GetHUD (Game|GetPlayerController 0))))
  (Default|CreateBossLifeBar _asbp_custom_hud self))

(event Custom|Attack
  (Animation|Montage|PlayMontage (Variables|Character|GetMesh) "/Game/InfinityBladeWarriors/Character/RetargetedAnimations/Other/AM_Magic_Attack_2.AM_Magic_Attack_2"))

(event Custom|invoke
  (Animation|Montage|PlayMontage (Variables|Character|GetMesh) "/Game/InfinityBladeWarriors/Character/RetargetedAnimations/Other/AM_Invoke.AM_Invoke"))

(event EventBeginPlay
  (|CallParentFunction)
  (bind _asabp_enemy (Utilities|Casting|CastToABP_Enemy (Components|SkeletalMesh|GetAnimInstance (Variables|Character|GetMesh))))
  (EventDispatchers|BindEventtoOnStartAttack _asabp_enemy (EventDispatchers|CreateEvent :!event SpawnBullets))
  (EventDispatchers|BindEventtoOnEndAttack _asabp_enemy (EventDispatchers|CreateEvent :!event MoveBullets))
  (EventDispatchers|BindEventtoOnInvkeEnemies _asabp_enemy (EventDispatchers|CreateEvent :!event InvokEnemies))
  (Transformation|SetRelativeLocation (Variables|Default|GetBox) (Variables|Default|GetTriggerPos) false false)
  (bind _output_get (Variables|Default|SetBlackBoard (AI|GetBlackboard (Pawn|GetController))))
  (AI|Components|Blackboard|SetValueasFloat _output_get (Variables|Default|GetCooldown) (Variables|Default|GetRateOfFire))
  (AI|Components|Blackboard|SetValueasFloat _output_get (Variables|Default|GetCooldownInvoke) 1e+01))

(event Collision|EventActorBeginOverlap
  (params (OtherActor :type Actor%20Object%20Reference)))

(event EventTick
  (params (DeltaSeconds :type Float%20%28single-precision%29)))

(fn ConstructionScript
  (|CallParentFunction))

(fn SpawnBullets
  (for _index (range 0 (Variables|Default|GetBulletAmount))
    (bind _randomlocation (Class|NavigationSystemV1|GetRandomLocationinNavigableRadius (Transformation|GetActorLocation) 2e+02 0 0))
    (bind _returnvalue (Game|SpawnActorfromClass "/Game/Parcial3/Enemy/Projectile/BP_EnemyBoss_Projectile.BP_EnemyBoss_Projectile_C" (Math|Transform|MakeTransform (Math|Vector|MakeVector (+ (.x _randomlocation) 8e+01) (.y _randomlocation) (+ (.z (Transformation|GetActorLocation)) 1e+02)) "0, 0, 0" "1.000000,1.000000,1.000000") "Undefined" 0 0))
    (Utilities|Array|SetArrayElem (Variables|Default|GetTarget) _index _returnvalue)))

(fn MoveBullets
  (bind _returnvalue (Game|GetPlayerCharacter 0))
  (bind _returnvalue_2 (Transformation|GetActorLocation _returnvalue))
  (for _array_element (Variables|Default|GetTarget)
    (Game|Components|ProjectileMovement|SetVelocityinLocalSpace (Variables|/Game/Parcial3/Enemy/Projectile/BP_EnemyBoss_Projectile.BP_EnemyBoss_Projectile_C|GetProjectileMovement _array_element) (* (Math|Vector|Normalize (- _returnvalue_2 (Transformation|GetActorLocation _array_element))) (Variables|Default|GetForce)))
    (Transformation|SetActorRotation _array_element (Math|Rotator|FindLookatRotation (Transformation|GetActorLocation _array_element) _returnvalue_2))))

(fn InvokEnemies
  (for _index (range 0 (Variables|Default|GetEnemiesAmount))
    (bind _randomlocation (Class|NavigationSystemV1|GetRandomLocationinNavigableRadius (Transformation|GetActorLocation) 5e+02 0 0))
    (bind _returnvalue (Game|SpawnActorfromClass "/Game/Parcial2/Enemies/EnemyMelee/BP_Enemy_Melee.BP_Enemy_Melee_C" (Math|Conversions|ToTransform(Vector) (+ _randomlocation "100.000000,0,0.000000")) "Undefined" 0 0))
    (bind _asbp_waypoints_component (Utilities|Casting|CastToBP_WaypointsComponent (Variables|/Game/Parcial2/Enemies/EnemyMelee/BP_Enemy_Melee.BP_Enemy_Melee_C|GetBP_WaypointsComponent _returnvalue)))
    (Variables|/Game/Parcial2/Components/BP_WaypointsComponent.BP_WaypointsComponent_C|SetWayPoints _asbp_waypoints_component (Utilities|Array|MakeArray (.RandomLocation (Class|NavigationSystemV1|GetRandomPointinNavigableRadius _randomlocation 5e+02 0 0)) (.RandomLocation (Class|NavigationSystemV1|GetRandomPointinNavigableRadius _randomlocation 5e+02 0 0))))
    (Utilities|Array|SetArrayElem (Variables|/Game/Parcial3/Compoent/BP_Spawn_Component.BP_Spawn_Component_C|GetactorsToSpawn (Variables|Default|GetBP_Spawn_Component)) _index (Utilities|GetClass _returnvalue))
    (Development|PrintString "te invoke")))