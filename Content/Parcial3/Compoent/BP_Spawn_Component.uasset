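; Actor component that spawns one of two actor classes, chosen at random, near its owning actor.
; BeginPlay rolls a random float against Probability once, selecting index 0 of ActorsToSpawn when the roll is higher and index 1 otherwise.
; RandomSpawnTwoActors spawns that stored choice at the owner's location plus a given offset, so repeated calls yield the same class.
; The SpawnActor function and Tick are empty.
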(event EventBeginPlay
  (bind _output_get (Variables|Default|SetRandoom%20Float (Math|Random|RandomFloat)))
  (if (> _output_get (Variables|Default|Getprobability))
    (Variables|Default|Setitem 0)
    (else
      (Variables|Default|Setitem 1))))

(event EventTick
  (params (DeltaSeconds :type Float%20%28single-precision%29)))

(fn RandomSpawnTwoActors
  (params (OffsetSpawn :type Vector))
  (Game|SpawnActorfromClass (Utilities|Array|Get(acopy) (Variables|Default|GetactorsToSpawn) (Variables|Default|Getitem)) (Math|Conversions|ToTransform(Vector) (+ OffsetSpawn (.location (Transformation|GetActorTransform (Components|GetOwner))))) "Undefined" 0 0))

(fn SpawnActor)