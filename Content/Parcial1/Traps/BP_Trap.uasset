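; BP_Trap is a trap actor that damages the first-person character when it enters the Radius collider.
; An overlap while the trap is down sets TrapUp and plays the TrapSetUp timeline, which clears the flag on finish.
; Whether the trap is up or down, each overlap applies truncated Damage through the character's BPHealthComponent and plays trap and damage sounds.
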(event OnComponentBeginOverlap(Radius)
  (params (OverlappedComponent :type Primitive%20Component%20Object%20Reference) (OtherActor :type Actor%20Object%20Reference) (OtherComp :type Primitive%20Component%20Object%20Reference) (OtherBodyIndex :type Integer) (bFromSweep :type Boolean) (SweepResult :type Hit%20Result%20Structure%20%28by%20ref%29))
  (bind _asbp_first_person_character (Utilities|Casting|CastToBP_FirstPersonCharacter OtherActor))
  (if (Variables|Default|GetTrapUp)
    (Default|TakeDamage (Variables|/Game/FirstPerson/Blueprints/BP_FirstPersonCharacter.BP_FirstPersonCharacter_C|GetBP_HealthComponent _asbp_first_person_character) (Math|Float|Truncate (Variables|Default|GetDamage)) :!label _label)
    (Utilities|FlowControl|Sequence
      (:then_0
        (Audio|PlaySound2D "/Game/Sounds/Trap_Cue.Trap_Cue" 1.0 1.0 0.0 0 0))
      (:then_1
        (Audio|PlaySound2D "/Game/Sounds/Damage_Cue.Damage_Cue" 1.0 1.0 0.0 0 0)))
    (else
      (Utilities|FlowControl|Sequence
        (:then_0
          (Variables|Default|SetTrapUp true)
          (Timeline|TrapSetUp Play
            (:Finished
              (Variables|Default|SetTrapUp false))))
        (:then_1
          (goto _label))))))

(fn ConstructionScript)