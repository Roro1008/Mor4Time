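; BP_LaserMove is a moving laser hazard that damages the first-person character on contact.
; The construction script builds a relative two-point InterpToMovement path from its origin to Destiny, using Speed as the travel duration.
; When Cube1 begins overlapping a BP_FirstPersonCharacter, it calls that character's TakeDamage with the truncated Damage value.
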(event OnComponentBeginOverlap(Cube1)
  (params (OverlappedComponent :type Primitive%20Component%20Object%20Reference) (OtherActor :type Actor%20Object%20Reference) (OtherComp :type Primitive%20Component%20Object%20Reference) (OtherBodyIndex :type Integer) (bFromSweep :type Boolean) (SweepResult :type Hit%20Result%20Structure%20%28by%20ref%29))
  (bind _asbp_first_person_character (Utilities|Casting|CastToBP_FirstPersonCharacter OtherActor))
  (Default|TakeDamage _asbp_first_person_character (Math|Float|Truncate (Variables|Default|GetDamage))))

(fn ConstructionScript
  (Variables|/Script/Engine.InterpToMovementComponent|SetDuration (Variables|Default|GetInterpToMovement) (Variables|Default|GetSpeed))
  (Class|InterptoMovementComponent|AddControlPointPosition (Variables|Default|GetInterpToMovement) "0, 0, 0" true)
  (Class|InterptoMovementComponent|AddControlPointPosition (Variables|Default|GetInterpToMovement) (Variables|Default|GetDestiny) true))