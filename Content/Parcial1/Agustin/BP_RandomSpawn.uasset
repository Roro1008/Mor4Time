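; BP_RandomSpawn is a breakable object that dissolves when hit by a first-person projectile and then spawns actors in its place.
; BeginPlay gives the Cube a dynamic M_Fade material instance with its fade parameter initialised.
; A projectile overlap plays a wood-breaking sound and a timeline that animates the fade amount.
; When the timeline finishes, BPSpawnComponent spawns the actors and the object destroys itself.
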(event OnComponentBeginOverlap(Cube)
  (params (OverlappedComponent :type Primitive%20Component%20Object%20Reference) (OtherActor :type Actor%20Object%20Reference) (OtherComp :type Primitive%20Component%20Object%20Reference) (OtherBodyIndex :type Integer) (bFromSweep :type Boolean) (SweepResult :type Hit%20Result%20Structure%20%28by%20ref%29))
  (Utilities|Casting|CastToBP_FirstPersonProjectile OtherActor)
  (Utilities|FlowControl|Sequence
    (:then_0
      (bind _newtrack_0 (Timeline|Timeline_0 Play)
        (:Update
          (Rendering|Material|SetScalarParameterValue (Variables|Default|GetDynamicMaterial) "Fade Amount" _newtrack_0 :!class /Script/Engine.MaterialInstanceDynamic))
        (:Finished
          (Utilities|Casting|CastToBP_FirstPersonProjectile OtherActor)
          (Default|SpawnActors (Variables|Default|GetBP_Spawn_Component))
          (Actor|DestroyActor))))
    (:then_1
      (Audio|PlaySound2D "/Game/Sounds/Wood_breaking_Cue.Wood_breaking_Cue" 1.0 1.0 0.0 0 0))))

(event EventBeginPlay
  (bind _returnvalue (Rendering|Material|CreateDynamicMaterialInstance (Variables|Default|GetCube) 0 "/Game/Parcial1/BP/M_Fade.M_Fade" "None" :!class /Script/Engine.PrimitiveComponent))
  (bind _output_get (Variables|Default|SetDynamicMaterial _returnvalue))
  (Rendering|Material|SetScalarParameterValue _output_get "Fade Amount" -1.0 :!class /Script/Engine.MaterialInstanceDynamic))

(fn ConstructionScript)