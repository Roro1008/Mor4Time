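; BP_VictoryTrigger is a goal volume that ends the game in victory when the player touches it.
; A Cube overlap casts to BP_FirstPersonCharacter, then calls Victory on its BP_CustomPC controller.
; From BeginPlay, a FlipFlop alternately plays and reverses the FadeAnimation timeline, looping through its Finished output.
; The timeline pulses the cube's "Starting" material parameter between MinFade and MaxFade.
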(event OnComponentBeginOverlap(Cube)
  (params (OverlappedComponent :type Primitive%20Component%20Object%20Reference) (OtherActor :type Actor%20Object%20Reference) (OtherComp :type Primitive%20Component%20Object%20Reference) (OtherBodyIndex :type Integer) (bFromSweep :type Boolean) (SweepResult :type Hit%20Result%20Structure%20%28by%20ref%29))
  ;[1 1 1] Collision
  (bind _asbp_first_person_character (Utilities|Casting|CastToBP_FirstPersonCharacter OtherActor))
  (bind _asbp_custom_pc (Utilities|Casting|CastToBP_CustomPC (Pawn|GetController _asbp_first_person_character)))
  (Default|Victory _asbp_custom_pc))

(event EventBeginPlay
  ;[1 1 1] AnimateMaterial
  (Utilities|FlowControl|FlipFlop :!label _label
    (:A
      (bind _fadeeffect (Timeline|FadeAnimation Play)
        (:Update
          (Rendering|Material|SetScalarParameterValueonMaterials (Variables|Default|GetCube) "Starting" (Math|Float|Lerp (Variables|Default|GetMinFade) (Variables|Default|GetMaxFade) _fadeeffect)))
        (:Finished
          (goto _label))))
    (:B
      (Timeline|FadeAnimation Reverse))))

(fn ConstructionScript)