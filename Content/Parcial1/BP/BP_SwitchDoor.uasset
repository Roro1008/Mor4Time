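; BP_SwitchDoor is a door that opens once enough pressure switches are active at the same time.
; SwitchActivate and SwitchDeactivate adjust the active count and compare it to the required number.
; The DoorActivate timeline then plays or reverses to drive the door's relative Z location.
; A 2D sliding sound plays on every switch change, even when the count stays on the same side of the threshold.
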(event Custom|SwitchActivate
  (Math|Integer|IncrementInt (Variables|Default|GetPressureSwitchesActive)
    (:%20%20
      (if (>= (Variables|Default|GetPressureSwitchesActive) (Variables|Default|GetPressureSwitchesNeeded))
        (Utilities|FlowControl|Sequence
          (:then_0
            (bind _doorposition (Timeline|DoorActivate Play)
              (:Update
                (Transformation|SetRelativeLocation (Variables|Default|GetDoor) (Math|Vector|MakeVector 0.0 0.0 _doorposition) false false))))
          (:then_1
            (Audio|PlaySound2D "/Game/Sounds/SlidingSound_Cue.SlidingSound_Cue" 1.0 1.0 0.0 0 0 :!label _label)))
        (else
          (Utilities|FlowControl|Sequence
            (:then_0
              (Timeline|DoorActivate Reverse))
            (:then_1
              (goto _label))))))))

(event Custom|SwitchDeactivate
  (Math|Integer|DecrementInt (Variables|Default|GetPressureSwitchesActive)
    (:%20%20
      (if (>= (Variables|Default|GetPressureSwitchesActive) (Variables|Default|GetPressureSwitchesNeeded))
        (Utilities|FlowControl|Sequence
          (:then_0
            (bind _doorposition (Timeline|DoorActivate Play)
              (:Update
                (Transformation|SetRelativeLocation (Variables|Default|GetDoor) (Math|Vector|MakeVector 0.0 0.0 _doorposition) false false))))
          (:then_1
            (Audio|PlaySound2D "/Game/Sounds/SlidingSound_Cue.SlidingSound_Cue" 1.0 1.0 0.0 0 0 :!label _label)))
        (else
          (Utilities|FlowControl|Sequence
            (:then_0
              (Timeline|DoorActivate Reverse))
            (:then_1
              (goto _label))))))))

(event EventBeginPlay)

(event Collision|EventActorBeginOverlap
  (params (OtherActor :type Actor%20Object%20Reference)))

(event EventTick
  (params (DeltaSeconds :type Float%20%28single-precision%29)))

(fn ConstructionScript)