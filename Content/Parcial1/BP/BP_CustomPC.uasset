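; Player controller that links the first-person character to the custom HUD and triggers the end-of-level screens.
; On possess, it casts the pawn and binds handlers to the health component's life-change and death events, plus the character's rifle-obtained and bullet-count events.
; Victory and Defeat functions tell the HUD to create the matching screen, with Victory passing along the level target.
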(event Custom|BindDamageComponent
  (params (Player :type BP%20First%20Person%20Character%20Object%20Reference) (HUD :type BP%20Custom%20HUD%20Object%20Reference))
  (bind _bp_healthcomponent (Variables|/Game/FirstPerson/Blueprints/BP_FirstPersonCharacter.BP_FirstPersonCharacter_C|GetBP_HealthComponent Player))
  ;[1 1 1] BindOnChangeHealh
  (EventDispatchers|BindEventtoOnLifeChange _bp_healthcomponent (EventDispatchers|CreateEvent HUD :!event PlayerChangeLife))
  (EventDispatchers|BindEventtoOnDeath _bp_healthcomponent (EventDispatchers|CreateEvent :!event Defeat)))

(event Custom|BindOnRifleObtained
  (params (Player :type BP%20First%20Person%20Character%20Object%20Reference) (HUD :type BP%20Custom%20HUD%20Object%20Reference))
  ;[1 1 1] BindOnRifleObtained
  (EventDispatchers|BindEventtoOnRifleObtained Player (EventDispatchers|CreateEvent HUD :!event CreateBulletWidget)))

(event Custom|BindOnChangeBullets
  (params (Player :type BP%20First%20Person%20Character%20Object%20Reference) (HUD :type BP%20Custom%20HUD%20Object%20Reference))
  ;[1 1 1] BindOnChangeBullets
  (EventDispatchers|BindEventtoOnBulletsValueChange Player (EventDispatchers|CreateEvent HUD :!event PlayerUpdateBullets)))

(event EventPossess
  (params (PossessedPawn :type Pawn%20Object%20Reference))
  (bind _returnvalue (HUD|GetHUD))
  (bind _asbp_custom_hud (Utilities|Casting|CastToBP_CustomHUD _returnvalue))
  ;[1 1 1] OnPossess
  (bind _asbp_first_person_character (Utilities|Casting|CastToBP_FirstPersonCharacter PossessedPawn))
  (CallFunction|BindDamageComponent _asbp_first_person_character _asbp_custom_hud)
  (CallFunction|BindonRifleObtained _asbp_first_person_character _asbp_custom_hud)
  (CallFunction|BindonChangeBullets _asbp_first_person_character _asbp_custom_hud))

(fn ConstructionScript)

(fn Victory
  (params (LevelTarget :type World%20Soft%20Object%20Reference))
  (bind _asbp_custom_hud (Utilities|Casting|CastToBP_CustomHUD (HUD|GetHUD)))
  (Default|CreateVictoryScreen _asbp_custom_hud LevelTarget))

(fn Defeat
  (bind _asbp_custom_hud (Utilities|Casting|CastToBP_CustomHUD (HUD|GetHUD)))
  (Default|CreateDefeatScreen _asbp_custom_hud))