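; BP_Enemy is an enemy actor that configures itself from a data table and fires projectiles on a repeating timer.
; On BeginPlay it looks up its DT_Enemies row by its class display name, storing max life and damage and setting the name widget's text.
; A looping timer at the row's rate of fire drives spawning of BP_FirstPersonProjectile at the actor's own transform, with no aiming.
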(event Custom|CustomEvent_0
  (Game|SpawnActorfromClass "/Game/FirstPerson/Blueprints/BP_FirstPersonProjectile.BP_FirstPersonProjectile_C" (Transformation|GetActorTransform) "Undefined" 0 0))

(event EventBeginPlay
  (Utilities|FlowControl|Sequence
    (:then_0
      (bind _returnvalue (Utilities|GetDataTableRow "/Game/Parcial2/DT_Enemies.DT_Enemies" (Utilities|String|StringToName (Utilities|GetClassDisplayName (Utilities|GetClass self))))
        (:then
          (bind _output_get (Variables|Default|SetEnemyData _returnvalue))
          (bind _aswbp_name (Utilities|Casting|CastToWBP_Name (UserInterface|GetWidget (Variables|Default|GetWidget))))
          (Default|SetName _aswbp_name (.Name (Utilities|Struct|BreakFEnemy _output_get)))
          (Variables|Default|SetMax%20Life (.MaxLife (Utilities|Struct|BreakFEnemy _output_get)))
          (Variables|Default|SetDamage (.Damage (Utilities|Struct|BreakFEnemy _output_get))))))
    (:then_1
      (Utilities|Time|SetTimerbyEvent (EventDispatchers|CreateEvent :!event Custom|CustomEvent_0) (.rateoffire (Variables|Default|GetEnemyData)) true))))

(fn ConstructionScript)