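; Health component that tracks an owner's current and maximum health and handles damage, healing and death.
; It initializes health to the maximum on BeginPlay and again whenever the maximum is changed.
; Damage and healing are clamped and broadcast through dispatchers, with damage also playing a 2D sound.
; Reaching zero sets a death flag that blocks further damage and fires OnDeath, while Heal does not check that flag.
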(event EventBeginPlay
  (CallFunction|Initialize))

(fn TakeDamage
  (params (Damage :type Integer))
  (bind _maxhealth (Variables|Default|GetMaxHealth))
  (if (not (Variables|Default|GetIsDeath))
    (bind _output_get (Variables|Default|SetCurrentHeatlh (Math|Integer|Clamp(Integer) (- (Variables|Default|GetCurrentHeatlh) Damage) 0 _maxhealth)))
    (Default|CallOnLifeChange _output_get _maxhealth)
    (Default|CallOnTakeDamage)
    (Audio|PlaySound2D (Variables|Default|GetTakeDamageSound) 1.0 1.0 0.0 0 0)
    (if (<= _output_get 0)
      (CallFunction|Death))))

(fn Death
  (Variables|Default|SetIsDeath true)
  (Default|CallOnDeath))

(fn Heal
  (params (HealAmmount :type Integer))
  (bind _maxhealth (Variables|Default|GetMaxHealth))
  (bind _output_get (Variables|Default|SetCurrentHeatlh (Math|Integer|Clamp(Integer) (+ HealAmmount (Variables|Default|GetCurrentHeatlh)) 0 _maxhealth)))
  (Default|CallOnLifeChange _output_get _maxhealth)
  (Default|CallOnHeal))

(fn SetMaxLife
  (params (NewMaxLife :type Integer))
  (Variables|Default|SetMaxHealth NewMaxLife)
  (CallFunction|Initialize))

(fn Initialize
  (bind _maxhealth (Variables|Default|GetMaxHealth))
  (bind _output_get (Variables|Default|SetCurrentHeatlh _maxhealth))
  (Default|CallOnLifeChange _output_get _maxhealth))