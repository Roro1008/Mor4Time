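; BP_WaypointsComponent stores a list of patrol waypoints and hands out the next one for its owning actor to move toward.
; GetNextPatrolPoint steps an index by a direction sign, then either restarts at the first point when IsCycle is set or reverses direction to ping-pong along the list.
; RecalculatePatrolPoints adds the owner's location to every waypoint in place, turning relative offsets into world positions.
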(fn GetNextPatrolPoint
  (if (or (>= (+ (Variables|Default|GetCurrentPatrolIndex) (Variables|Default|GetSign)) (Utilities|Array|Length (Variables|Default|GetWayPoints))) (<= (+ (Variables|Default|GetCurrentPatrolIndex) (Variables|Default|GetSign)) -1))
    (if (Variables|Default|GetIsCycle)
      (Variables|Default|SetCurrentPatrolIndex 0)
      (else
        (bind _output_get (Variables|Default|SetSign (* (Variables|Default|GetSign) -1)))
        (Variables|Default|SetCurrentPatrolIndex (+ (Variables|Default|GetCurrentPatrolIndex) _output_get))))
    (else
      (Variables|Default|SetCurrentPatrolIndex (+ (Variables|Default|GetCurrentPatrolIndex) (Variables|Default|GetSign)))))
  (return (Utilities|Array|Get(acopy) (Variables|Default|GetWayPoints) (Variables|Default|GetCurrentPatrolIndex))))

(fn RecalculatePatrolPoints
  (for (_array_element _array_index) (Variables|Default|GetWayPoints)
    (Utilities|Array|SetArrayElem (Variables|Default|GetWayPoints) _array_index (+ _array_element (Transformation|GetActorLocation (Components|GetOwner))))))