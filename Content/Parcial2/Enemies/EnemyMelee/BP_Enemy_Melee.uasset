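; Melee enemy character that patrols, senses the first-person player and damages them through a toggled hit collider.
; BeginPlay feeds fire rate to the Blackboard as WaitTime, and AI perception writes player sight and target keys.
; Patrol points become world positions offset from spawn, and GetNextPatrolPoint steps through them in a loop or ping-pong.
; The collider deals one hit, then deactivates; the attack montage chain that would activate it is unconnected.
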(event OnTargetPerceptionUpdated(AIPerception)
  (params (Actor :type Actor%20Object%20Reference) (Stimulus :type AI%20Stimulus%20Structure))
  ;[1 1 1] AIPerception
  (bind _asbp_first_person_character (Utilities|Casting|CastToBP_FirstPersonCharacter Actor))
  (AI|Components|Blackboard|SetValueasBool (Variables|Default|GetBlackBoard) (Variables|Default|GetInSightKey) (.bSuccessfullySensed (Utilities|Struct|BreakAIStimulus Stimulus)))
  (AI|Components|Blackboard|SetValueasObject (Variables|Default|GetBlackBoard) (Variables|Default|GetTargetKey) _asbp_first_person_character))

(event OnComponentBeginOverlap(DamageCollision)
  (params (OverlappedComponent :type Primitive%20Component%20Object%20Reference) (OtherActor :type Actor%20Object%20Reference) (OtherComp :type Primitive%20Component%20Object%20Reference) (OtherBodyIndex :type Integer) (bFromSweep :type Boolean) (SweepResult :type Hit%20Result%20Structure%20%28by%20ref%29))
  ;[1 1 1] Damage
  (if (Components|Activation|IsActive (Variables|Default|GetDamageCollision))
    (bind _asbp_first_person_character (Utilities|Casting|CastToBP_FirstPersonCharacter OtherActor))
    (Default|TakeDamage (Variables|/Game/FirstPerson/Blueprints/BP_FirstPersonCharacter.BP_FirstPersonCharacter_C|GetBP_HealthComponent _asbp_first_person_character) (Variables|Default|GetDamage))
    (CallFunction|ActiveDamageCollider false)))

(event Custom|VisualizeHealth
  (params (CurrentHealth :type Integer) (MaxHealth :type Integer))
  (Development|PrintString (Utilities|String|Append (Utilities|String|ToString(Integer) CurrentHealth) "/" (Utilities|String|ToString(Integer) MaxHealth)) true true "(R=1.000000,G=0.000000,B=0.572170,A=1.000000)" 1.5))

(event EventBeginPlay
  ;[1 1 1] BeginPlay
  (|CallParentFunction)
  (bind _output_get (Variables|Default|SetBlackBoard (AI|GetBlackboard (Pawn|GetController))))
  (Audio|Parameter|SetFloatParameter _output_get "WaitTime" (.RateOfFire (Utilities|Struct|BreakFEnemy (Variables|Default|GetEnemy%20Data))) :!class /Script/AudioExtensions.AudioParameterControllerInterface)
  (CallFunction|RecalculatePatrolPoints)
  (CallFunction|ActiveDamageCollider false)
  (EventDispatchers|BindEventtoOnLifeChange (Variables|Default|GetBP_HealthComponent) (EventDispatchers|CreateEvent :!event Custom|VisualizeHealth)))

(event EventTick
  (params (DeltaSeconds :type Float%20%28single-precision%29)))

(fn ConstructionScript
  (|CallParentFunction))

(fn ActiveDamageCollider
  (params (Active :type Boolean))
  (Components|Activation|SetActive (Variables|Default|GetDamageCollision) Active true))

(fn RecalculatePatrolPoints
  (for (_array_element _array_index) (Variables|Default|GetPatrolPoints)
    (Utilities|Array|SetArrayElem (Variables|Default|GetPatrolPoints) _array_index (+ _array_element (Transformation|GetActorLocation)))))

(fn GetNextPatrolPoint
  (if (or (>= (+ (Variables|Default|GetCurrentPatrolIndex) (Variables|Default|GetSign)) (Utilities|Array|Length (Variables|Default|GetPatrolPoints))) (<= (+ (Variables|Default|GetCurrentPatrolIndex) (Variables|Default|GetSign)) -1))
    (if (Variables|Default|GetIsCycle)
      (Variables|Default|SetCurrentPatrolIndex 0)
      (else
        (bind _output_get (Variables|Default|SetSign (* (Variables|Default|GetSign) -1)))
        (Variables|Default|SetCurrentPatrolIndex (+ (Variables|Default|GetCurrentPatrolIndex) _output_get))))
    (else
      (Variables|Default|SetCurrentPatrolIndex (+ (Variables|Default|GetCurrentPatrolIndex) (Variables|Default|GetSign)))))
  (return (Utilities|Array|Get(acopy) (Variables|Default|GetPatrolPoints) (Variables|Default|GetCurrentPatrolIndex))))