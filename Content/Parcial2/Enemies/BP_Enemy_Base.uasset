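; Base enemy Blueprint that configures itself from data and reacts to damage and death.
; On BeginPlay it looks up its EnemyType name in DT_Enemies to set max life, skeletal mesh, fire rate and damage, printing an error if missing.
; It then binds to its health component's damage and death delegates.
; Hits play a montage while alive; death deactivates the capsule, plays a death montage and destroys the actor on completion.
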(event Custom|TakeDamage
  ;[1 1 1] TakeDamage
  (if (not (Variables|Default|GetIsDeath))
    (Animation|Montage|PlayMontage (Variables|Character|GetMesh) (Variables|Default|GetGetHitMontage))))

(event Custom|DeathBehavior
  ;[1 1 1] Death
  (Variables|Default|SetIsDeath true)
  (Components|Activation|Deactivate (Variables|Collision|GetCapsuleComponent))
  (Animation|Montage|PlayMontage (Variables|Character|GetMesh) (Variables|Default|GetDeathMontage)
    (:OnCompleted
      (Actor|DestroyActor))))

(event EventBeginPlay
  (bind _enemytype (Variables|Default|GetEnemyType))
  (bind _bp_healthcomponent (Variables|Default|GetBP_HealthComponent))
  (bind _returnvalue (Utilities|String|EnumtoString _enemytype))
  ;[1 1 1] GetData
  (bind _returnvalue_2 (Utilities|GetDataTableRow "/Game/Parcial2/DT_Enemies.DT_Enemies" (Utilities|String|StringToName _returnvalue))
    (:then
      (bind _output_get (Variables|Default|SetEnemy%20Data _returnvalue_2))
      (Utilities|FlowControl|Sequence
        (:then_0
          ;[1 1 1] SetMaxLife
          (Default|SetMaxLife (Variables|Default|GetBP_HealthComponent) (Math|Float|Truncate (.MaxLife (Utilities|Struct|BreakFEnemy _output_get))))
          ;[1 1 1] SetMesh
          (Class|SkinnedMeshComponent|SetSkeletalMesh (Variables|Character|GetMesh) (.Mesh (Utilities|Struct|BreakFEnemy _output_get)) true)
          ;[1 1 1] SetOtherParams
          (Variables|Default|SetRateOfFire (.RateOfFire (Utilities|Struct|BreakFEnemy _output_get)))
          (Variables|Default|SetDamage (Math|Float|Truncate (.Damage (Utilities|Struct|BreakFEnemy _output_get)))))
        (:then_1
          ;[1 1 1] Bind HealthComponent
          (EventDispatchers|BindEventtoOnTakeDamage _bp_healthcomponent (EventDispatchers|CreateEvent :!event Custom|TakeDamage))
          (EventDispatchers|BindEventtoOnDeath _bp_healthcomponent (EventDispatchers|CreateEvent :!event Custom|DeathBehavior)))))
    (:RowNotFound
      (Development|PrintString (Utilities|String|Append "Enemy Type: " _returnvalue " NOT FOUND") true true "(R=0.000000,G=0.660000,B=1.000000,A=1.000000)" 3.0))))

(fn ConstructionScript)