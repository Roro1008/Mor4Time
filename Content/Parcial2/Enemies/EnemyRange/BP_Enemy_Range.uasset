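; Ranged enemy character that patrols waypoints and attacks the player with projectiles.
; BeginPlay feeds patrol points to the waypoint component, writes fire rate to the Blackboard and binds to the anim instance's attack-start event.
; AI perception updates the Blackboard's target and sight flag.
; Attack plays a montage while flagging the Blackboard, and Bullet spawns a damage-carrying projectile from the right-hand socket.
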(event OnTargetPerceptionUpdated(AIPerception)
  (params (Actor :type Actor%20Object%20Reference) (Stimulus :type AI%20Stimulus%20Structure))
  (bind _self self)
  (bind _returnvalue (AI|GetAIController _self))
  (bind _returnvalue_2 (AI|GetBlackboard _returnvalue))
  (bind _asbp_first_person_character (Utilities|Casting|CastToBP_FirstPersonCharacter Actor))
  (AI|Components|Blackboard|SetValueasBool _returnvalue_2 (Utilities|Name|MakeLiteralName "IsTargetInSight") (.bSuccessfullySensed (Utilities|Struct|BreakAIStimulus Stimulus)))
  (AI|Components|Blackboard|SetValueasObject _returnvalue_2 (Utilities|Name|MakeLiteralName "TargetActor") _asbp_first_person_character))

(event Custom|Attack
  (AI|Components|Blackboard|SetValueasBool (Variables|Default|GetBlackBoard) (Variables|Default|GetIsAttack) true)
  (Animation|Montage|PlayMontage (Variables|Character|GetMesh) "/Game/InfinityBladeWarriors/Character/RetargetedAnimations/Other/AM_Attack.AM_Attack"
    (:OnCompleted
      (AI|Components|Blackboard|SetValueasBool (Variables|Default|GetBlackBoard) (Variables|Default|GetIsAttack) false))))

(event EventBeginPlay
  (bind _bp_waypointscomponent (Variables|Default|GetBP_WaypointsComponent))
  (|CallParentFunction)
  (Variables|Default|SetBlackBoard (AI|GetBlackboard (Pawn|GetController)))
  (Variables|/Game/Parcial2/Components/BP_WaypointsComponent.BP_WaypointsComponent_C|SetWayPoints _bp_waypointscomponent (Variables|Default|GetPatrolPoints))
  (Default|RecalculatePatrolPoints _bp_waypointscomponent)
  (AI|Components|Blackboard|SetValueasFloat (Variables|Default|GetBlackBoard) (Utilities|Name|MakeLiteralName "Wait") (Variables|Default|GetRateOfFire))
  (bind _asabp_enemy (Utilities|Casting|CastToABP_Enemy (Components|SkeletalMesh|GetAnimInstance (Variables|Character|GetMesh))))
  (EventDispatchers|BindEventtoOnStartAttack _asabp_enemy (EventDispatchers|CreateEvent :!event Bullet)))

(fn ConstructionScript
  (|CallParentFunction))

(fn Bullet
  (bind _returnvalue (Game|SpawnActorfromClass "/Game/Parcial2/Enemies/EnemyRange/BP_Enemy_Range_Projectile.BP_Enemy_Range_Projectile_C" (Math|Transform|MakeTransform (Transformation|GetSocketLocation (Variables|Character|GetMesh) "hand_r") (Transformation|GetActorRotation)) "Undefined" 0 0))
  (Variables|/Game/Parcial2/Enemies/EnemyRange/BP_Enemy_Range_Projectile.BP_Enemy_Range_Projectile_C|SetDamage _returnvalue (Variables|Default|GetDamage))
  (Development|PrintText "Hello"))