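; BP_Enemy_Melee is a melee enemy, derived from a parent class, that damages the first-person player on contact with its DamageCollision.
; The collider starts inactive via ActiveDamageCollider, and an overlap while active calls TakeDamage on the player's health component, then deactivates it.
; Its own health changes print as debug text.
; The delayed attack-montage chain that would activate the collider is disconnected, so nothing here enables damage.
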(event OnComponentBeginOverlap(DamageCollision)
  (params (OverlappedComponent :type Primitive%20Component%20Object%20Reference) (OtherActor :type Actor%20Object%20Reference) (OtherComp :type Primitive%20Component%20Object%20Reference) (OtherBodyIndex :type Integer) (bFromSweep :type Boolean) (SweepResult :type Hit%20Result%20Structure%20%28by%20ref%29))
  (if (Components|Activation|IsActive (Variables|Default|GetDamageCollision))
    (bind _asbp_first_person_character (Utilities|Casting|CastToBP_FirstPersonCharacter OtherActor))
    (Default|TakeDamage (Variables|/Game/FirstPerson/Blueprints/BP_FirstPersonCharacter.BP_FirstPersonCharacter_C|GetBP_HealthComponent _asbp_first_person_character) (Variables|Default|GetDamage))
    (CallFunction|ActiveDamageCollider false)))

(event Custom|CustomEvent_0
  (params (CurrentHealth :type Integer) (MaxHealth :type Integer))
  (Development|PrintString (Utilities|String|Append (Utilities|String|ToString(Integer) CurrentHealth) "/" (Utilities|String|ToString(Integer) MaxHealth)) true true "(R=1.000000,G=0.000000,B=0.572170,A=1.000000)" 1.5))

(event EventBeginPlay
  (|CallParentFunction)
  (CallFunction|ActiveDamageCollider false)
  (EventDispatchers|BindEventtoOnLifeChange (Variables|Default|GetBP_HealthComponent) (EventDispatchers|CreateEvent :!event Custom|CustomEvent_0)))

(event EventTick
  (params (DeltaSeconds :type Float%20%28single-precision%29)))

(fn ConstructionScript
  (|CallParentFunction))

(fn ActiveDamageCollider
  (params (Active :type Boolean))
  (Components|Activation|SetActive (Variables|Default|GetDamageCollision) Active true))